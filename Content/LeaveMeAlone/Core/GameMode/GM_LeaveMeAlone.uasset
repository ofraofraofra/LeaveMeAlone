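; Game mode for LeaveMeAlone that runs the match countdown and shows the end screen on timeout or player death.
; A looping one-second timer decrements GameTime and, at zero, stops itself and pauses the game.
; The player's LMAHealthComponent death event stops the timer and waits a second, without pausing.
; Both paths then show WBP_TimerOut with UI-only input and a visible cursor.
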(event Custom|CustomEvent_1
  (Utilities|Time|ClearandInvalidateTimerbyHandle (Variables|Default|GetGameTimerHandle))
  (Utilities|FlowControl|Delay 1.0)
  (bind _returnvalue (UserInterface|CreateWidget "/Game/LeaveMeAlone/Widgets/UI/WBP_TimerOut.WBP_TimerOut_C"))
  (UserInterface|Viewport|AddtoViewport _returnvalue 0)
  (bind _aspc_leave_me_alone (Utilities|Casting|CastToPC_LeaveMeAlone (Game|GetPlayerController 0)))
  (Input|SetInputModeUIOnly _aspc_leave_me_alone _returnvalue "DoNotLock" false)
  (Variables|/Script/Engine.PlayerController|SetbShowMouseCursor _aspc_leave_me_alone true))

(event Custom|CustomEvent
  (bind _output_get (Variables|Default|SetGameTime (- (Variables|Default|GetGameTime) 1)))
  (if (== _output_get 0)
    (Utilities|Time|ClearandInvalidateTimerbyHandle (Variables|Default|GetGameTimerHandle))
    (Game|SetGamePaused true)
    (bind _returnvalue (UserInterface|CreateWidget "/Game/LeaveMeAlone/Widgets/UI/WBP_TimerOut.WBP_TimerOut_C"))
    (UserInterface|Viewport|AddtoViewport _returnvalue 0)
    (bind _aspc_leave_me_alone (Utilities|Casting|CastToPC_LeaveMeAlone (Game|GetPlayerController 0)))
    (Input|SetInputModeUIOnly _aspc_leave_me_alone _returnvalue "DoNotLock" false)
    (Variables|/Script/Engine.PlayerController|SetbShowMouseCursor _aspc_leave_me_alone true)))

(event EventBeginPlay
  (Utilities|FlowControl|Sequence
    (:then_0
      (bind _returnvalue (Utilities|Time|SetTimerbyEvent (delegate Custom|CustomEvent) 1.0 true))
      (Variables|Default|SetGameTimerHandle _returnvalue))
    (:then_1
      (EventDispatchers|BindEventtoOnDeath (Actor|GetComponentbyClass (Game|GetPlayerCharacter 0) "/Script/LeaveMeAlone.LMAHealthComponent") (delegate Custom|CustomEvent_1)))))

(fn ConstructionScript)