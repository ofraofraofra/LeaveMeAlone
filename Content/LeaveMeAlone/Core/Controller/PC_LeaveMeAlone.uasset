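; Player controller for LeaveMeAlone that opens the pause menu when the Pause input is pressed.
; An OnPause flag guards against repeat presses; this graph sets it but never clears it.
; With a valid CH_Player pawn, it stops the LMAWeaponComponent firing, pauses the game and shows a WBP_Pause widget.
; It then switches input to UI-only focused on that widget and shows the mouse cursor.
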(event EventBeginPlay)

(event Input|ActionEvents|InputActionPause
  (params (Key :type Key%20Structure :default "None"))
  (:Pressed
    (if (not (Variables|Default|GetonPause))
      (Variables|Default|SetonPause true)
      (bind _asch_player (Utilities|Casting|CastToCH_Player (Game|Player|GetPlayerPawn 0)))
      (Utilities|IsValid _asch_player
        (:Is%20Valid
          (Class|LMAWeaponComponent|StopFire (Actor|GetComponentbyClass _asch_player "/Script/LeaveMeAlone.LMAWeaponComponent"))
          (Game|SetGamePaused true)
          (bind _returnvalue (UserInterface|CreateWidget "/Game/LeaveMeAlone/Widgets/UI/WBP_Pause.WBP_Pause_C"))
          (bind _output_get (Variables|Default|SetPause%20Widget _returnvalue))
          (UserInterface|Viewport|AddtoViewport _output_get 0)
          (Input|SetInputModeUIOnly self _returnvalue "DoNotLock" false)
          (Variables|Default|SetbShowMouseCursor true))))))

(fn ConstructionScript)